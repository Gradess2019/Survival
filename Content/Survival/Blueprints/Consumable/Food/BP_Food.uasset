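; BP_Food is a consumable food actor that applies a hunger-decreasing effect to whoever interacts with it.
; Interact applies GE_DecreaseHunger through the instigator's Ability System Component, then destroys the food.
; Without a valid component the food stays, though Interact returns true in both cases.
; Every tick, its TextRender rotates against the player camera's forward vector, keeping the label screen-facing.
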(event `self.ReceiveTick`
  (params (DeltaSeconds :type "Float (single-precision)"))
  (`SceneComponent.K2_SetWorldRotation` (`self.TextRender`) (`KismetMathLibrary.Conv_VectorToRotator` (`KismetMathLibrary.NegateVector` (`KismetMathLibrary.GetForwardVector` (`PlayerCameraManager.GetCameraRotation` (`GameplayStatics.GetPlayerCameraManager` 0))))) false false))

(fn `Interact`
  (params (Instigator :type "Actor Object Reference"))
  (returns (ReturnValue :type Boolean))
  (bind _returnvalue (`AbilitySystemBlueprintLibrary.GetAbilitySystemComponent` Instigator))
  (`/Engine/EditorBlueprintResources/StandardMacros.IsValid` _returnvalue
    (:`Is Valid`
      (`AbilitySystemComponent.BP_ApplyGameplayEffectToSelf` :`self` _returnvalue :`GameplayEffectClass` "/Game/Survival/Blueprints/AbilitySystem/Effects/GE_DecreaseHunger.GE_DecreaseHunger_C" :`Level` 1.0)
      (`self.K2_DestroyActor`)
      (return true))
    (:`Is Not Valid`
      (return true))))

(fn `UserConstructionScript`)