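; Gameplay ability for walking that raises the level of effects tagged Effect.Needs while WASD movement keys are held, without moving the character itself.
; On activation it listens for those keys, including already-held ones, and counts presses and releases.
; A DoOnce applies the level increase on the first press and sets the count to one.
; The ability ends when the count reaches zero, and its end event lowers the level again.
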(event `self.K2_ActivateAbility`
  (bind _pressed (`self.Pressed`))
  (`GLibAbilityTask_WaitForKeyInput.WaitForKeyInput` (`|MakeArray` "W" "A" "S" "D" :!type "Key Structure") true
    (:`Pressed`
      (`/Engine/EditorBlueprintResources/StandardMacros.IncrementInt` _pressed
        (:`  `
          (`/Engine/EditorBlueprintResources/StandardMacros.DoOnce` false
            (:`Completed`
              (`GLibGameplayEffectLibrary.AddGameplayEffectLevelByTags` (`self.GetAbilitySystemComponentFromActorInfo`) (struct :`GameplayTags` (struct :`(TagName` "Effect.Needs"))))
              (set `self.Pressed` 1))))))
    (:`Released`
      (bind _result (`/Engine/EditorBlueprintResources/StandardMacros.DecrementInt` _pressed)
        (:`  `
          (if (== _result 0)
            (`self.K2_EndAbility`)))))))

(event `self.K2_OnEndAbility`
  (params (bWasCancelled :type Boolean))
  (`GLibGameplayEffectLibrary.AddGameplayEffectLevelByTags` (`self.GetAbilitySystemComponentFromActorInfo`) (struct :`GameplayTags` (struct :`(TagName` "Effect.Needs"))) -1))