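; Movement ability that turns the player toward the mouse cursor every frame.
; BeginPlay caches the player controller from AbilityInfo and its controlled pawn.
; Tick deprojects the mouse into a line trace, then sets control rotation to look from the pawn at the hit location, or at the trace end when nothing blocks.
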(event `self.ReceiveBeginPlay`
  (bind _output_get (set `self.PlayerController` (`.PlayerController` (break `GameplayAbilityActorInfo` (`self.AbilityInfo`)))))
  (set `self.Pawn` (`Controller.K2_GetPawn` _output_get)))

(event `self.ReceiveTick`
  (params (DeltaSeconds :type "Float (single-precision)"))
  (bind (_worldlocation _worlddirection) (`PlayerController.DeprojectMousePositionToWorld` (`self.PlayerController`)))
  (bind _outhit (`KismetSystemLibrary.LineTraceSingle` :`Start` _worldlocation :`End` (+ _worldlocation (* _worlddirection 6000.0)) :`TraceChannel` "TraceTypeQuery4" :`DrawTime` 2.0))
  (`Controller.SetControlRotation` (`self.PlayerController`) (`KismetMathLibrary.FindLookAtRotation` (`self.K2_GetActorLocation` (`self.Pawn`)) (`KismetMathLibrary.SelectVector` (`.Location` (`GameplayStatics.BreakHitResult` _outhit)) (`.TraceEnd` (`GameplayStatics.BreakHitResult` _outhit)) (`GameplayStatics.BreakHitResult` _outhit)))))

(fn `UserConstructionScript`)