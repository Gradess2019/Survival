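; Base Gameplay Ability for survival character movement states, active while any WASD key is held.
; A key-wait task tracks pressed keys, and the first press applies a configurable movement effect plus a stat-decrease effect at a configurable level.
; Releasing the last key activates the Idle movement ability and ends this one, which removes both effects by handle.
; Unconnected nodes hold an alternative that adjusts the stat-decrease effect level by tag.
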(event `self.K2_ActivateAbility`
  (bind _pressedkeys (`self.PressedKeys`))
  (`self.K2_CommitAbility`)
  (bind (_asynctaskproxy _key) (`GLibAbilityTask_WaitForKeyInput.WaitForKeyInput` (`|MakeArray` "W" "A" "S" "D" :!type "Key Structure") true)
    (:`Pressed`
      (`BlueprintSetLibrary.Set_Add` _pressedkeys _key)
      (if (> (`BlueprintSetLibrary.Set_Length` (`self.PressedKeys`)) 0)
        (`/Engine/EditorBlueprintResources/StandardMacros.DoOnce` false
          (:`Completed`
            (bind _returnvalue (`self.BP_ApplyGameplayEffectToOwner` (`self.MovementEffectClass`)))
            (set `self.MovementEffect` _returnvalue)
            (bind _returnvalue_2 (`self.BP_ApplyGameplayEffectToOwner` "/Game/Survival/Blueprints/AbilitySystem/Effects/Stats/GE_DecreaseStats.GE_DecreaseStats_C" (`self.DecreaseStatsLevel`)))
            (set `self.DecreaseStatsEffect` _returnvalue_2)))))
    (:`Released`
      (`BlueprintSetLibrary.Set_Remove` _pressedkeys _key)
      (if (== (`BlueprintSetLibrary.Set_Length` (`self.PressedKeys`)) 0)
        (`GLibGASCharacter.ActivateAbility` (cast `SurvivalCharacter` (`self.GetOwningActorFromActorInfo`) :!pure true) (struct :`GameplayTags` (struct :`(TagName` "Movement.Idle"))))
        (`self.K2_EndAbility`)))))

(event `self.K2_OnEndAbility`
  (params (bWasCancelled :type Boolean))
  (`self.BP_RemoveGameplayEffectFromOwnerWithHandle` (`self.MovementEffect`))
  (`self.BP_RemoveGameplayEffectFromOwnerWithHandle` (`self.DecreaseStatsEffect`)))