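; GA_Idle is a movement gameplay ability that puts the owning actor into the Idle movement mode.
; On activation it commits, applies each gameplay effect in a class-to-level map to the owner, stores the handles, and sets the walk mode manager's current mode to Idle.
; When the ability ends it removes every stored effect handle with all stacks, so the effects last only as long as the ability.
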(event `self.K2_ActivateAbility`
  (`self.K2_CommitAbility`)
  (bind _keys (`BlueprintMapLibrary.Map_Keys` (`self.Gameplay Effect Class`)))
  (for _array_element _keys
    (bind _returnvalue (`self.BP_ApplyGameplayEffectToOwner` _array_element (`BlueprintMapLibrary.Map_Find` (`self.Gameplay Effect Class`) _array_element)))
    (`BlueprintSetLibrary.Set_Add` (`self.Effects`) _returnvalue))
  (set `WalkModeManagerComponent.CurrentMovementMode` "Idle" (`WalkModeManagerComponent.GetWalkModeManager` (`self.GetOwningActorFromActorInfo`))))

(event `self.K2_OnEndAbility`
  (params (bWasCancelled :type Boolean))
  (bind _result (`BlueprintSetLibrary.Set_ToArray` (`self.Effects`)))
  (for _array_element _result
    (`self.BP_RemoveGameplayEffectFromOwnerWithHandle` _array_element)))