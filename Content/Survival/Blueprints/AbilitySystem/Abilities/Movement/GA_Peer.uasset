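; GA_Peer is a movement gameplay ability that turns the player toward the mouse while active.
; Commit spawns a BP_RotatePlayerToMouse actor with the ability's actor info and stores it as PlayerRotator.
; Activation switches character movement from orient-to-movement to controller-desired rotation.
; On end, a valid rotator is destroyed and both rotation flags are set from the movement-component cast's success, rather than saved values.
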(event `self.K2_ActivateAbility`
  (bind (_returnvalue_owneractor _returnvalue_avataractor _returnvalue_playercontroller _returnvalue_abilitysystemcomponent _returnvalue_skeletalmeshcomponent _returnvalue_animinstance _returnvalue_movementcomponent) (break `GameplayAbilityActorInfo` (`self.GetActorInfo`)))
  (bind (_ascharacter_movement_component _bsuccess) (cast `CharacterMovementComponent` _returnvalue_movementcomponent :!pure true))
  (`self.K2_CommitAbility`)
  (set `CharacterMovementComponent.bOrientRotationToMovement` false _ascharacter_movement_component)
  (set `CharacterMovementComponent.bUseControllerDesiredRotation` true _ascharacter_movement_component))

(event `self.K2_OnEndAbility`
  (params (bWasCancelled :type Boolean))
  (bind (_returnvalue_owneractor _returnvalue_avataractor _returnvalue_playercontroller _returnvalue_abilitysystemcomponent _returnvalue_skeletalmeshcomponent _returnvalue_animinstance _returnvalue_movementcomponent) (break `GameplayAbilityActorInfo` (`self.GetActorInfo`)))
  (bind (_ascharacter_movement_component _bsuccess) (cast `CharacterMovementComponent` _returnvalue_movementcomponent :!pure true))
  (`/Engine/EditorBlueprintResources/StandardMacros.IsValid` (`self.PlayerRotator`)
    (:`Is Valid`
      (`Actor.K2_DestroyActor` (`self.PlayerRotator`))
      (set `CharacterMovementComponent.bOrientRotationToMovement` _bsuccess _ascharacter_movement_component)
      (set `CharacterMovementComponent.bUseControllerDesiredRotation` _bsuccess _ascharacter_movement_component))))

(event `self.K2_CommitExecute`
  (bind _returnvalue (`|SpawnActorFromClass` "/Game/Survival/Blueprints/AbilitySystem/Abilities/Movement/BP_RotatePlayerToMouse.BP_RotatePlayerToMouse_C" (`KismetMathLibrary.MakeTransform` (0.0 0.0 0.0)) "AlwaysSpawn" "OverrideRootScale" null (`self.GetActorInfo`) null))
  (set `self.PlayerRotator` _returnvalue))