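; BP_Door is an interactable door that toggles between open and closed.
; Interact flips the replicated Opened flag and reports success, without using the instigator.
; The flag's RepNotify snaps the mesh between two relative rotations with no interpolation, using the unrotated pose for the opened state.
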(fn `Interact`
  (params (Instigator :type "Actor Object Reference"))
  (returns (ReturnValue :type Boolean))
  (set `self.bOpened` (not (`self.bOpened`)))
  (return true))

(fn `OnRep_bOpened`
  (`SceneComponent.K2_SetRelativeRotation` (`self.Mesh`) (`KismetMathLibrary.SelectRotator` (struct) (struct :`Yaw` -90.0) (`self.bOpened`)) false false))

(fn `UserConstructionScript`
  (`parent.UserConstructionScript`))