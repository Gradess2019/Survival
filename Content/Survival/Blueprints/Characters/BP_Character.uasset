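; Player character Blueprint for a survival game, driving movement abilities and grid-based wall building from input.
; BeginPlay shows the HUD and ability-system debug display, then caches the WorldGrid and its WallBuilder.
; Walk, run and crouch activate tagged gameplay abilities, with run and crouch canceled on key release.
; Separate E-key events place a wall at the character's feet along its grid-aligned facing and save the grid; Escape quits.
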(event `self.ReceiveBeginPlay`
  (`KismetSystemLibrary.ExecuteConsoleCommand` "showdebug abilitysystem" null)
  (bind _returnvalue (`|CreateWidget` "/Game/Survival/Blueprints/Widgets/WBP_HUD.WBP_HUD_C"))
  (`UserWidget.AddToViewport` _returnvalue 0)
  (bind _returnvalue_2 (`GameplayStatics.GetActorOfClass` "/Script/Survival.WorldGrid"))
  (bind _output_get (set `self.WorldGrid` _returnvalue_2))
  (set `self.Wall` (`WorldGrid.WallBuilder` _output_get)))

(event `InputAction|WalkAction`
  (params (Key :type "Key Structure"))
  (:`Pressed`
    (`self.ActivateAbility` (struct :`GameplayTags` (struct :`(TagName` "Movement.Walk"))))))

(event `Key|E`
  (params (Key :type "Key Structure"))
  (:`Pressed`
    (`WallBuilder.CreateWall` (`self.Wall`) (- (`self.K2_GetActorLocation`) (`KismetMathLibrary.MakeVector` 0.0 0.0 (`.OutHalfHeight` (`CapsuleComponent.GetScaledCapsuleSize` (`self.CapsuleComponent`))))) (`GridLibrary.GetGridDirection` (`self.GetActorForwardVector`)))))

(event `Key|LeftShift`
  (params (Key :type "Key Structure"))
  (:`Pressed`
    (`self.ActivateAbility` (struct :`GameplayTags` (struct :`(TagName` "Movement.Run")))))
  (:`Released`
    (`self.CancelAbilityWithTags` (struct :`GameplayTags` (struct :`(TagName` "Movement.Run"))) (struct) null)))

(event `Key|RightMouseButton` :overrideparent false
  (params (Key :type "Key Structure"))
  (:`Pressed`
    (`self.ActivateAbility` (struct :`GameplayTags` (struct :`(TagName` "Movement.Crouch")))))
  (:`Released`
    (`self.CancelAbilityWithTags` (struct :`GameplayTags` (struct :`(TagName` "Movement.Crouch"))) (struct) null)))

(event `Key|Escape`
  (params (Key :type "Key Structure"))
  (:`Pressed`
    (`KismetSystemLibrary.QuitGame` null "Quit")))

(event `Key|E`
  (params (Key :type "Key Structure"))
  (:`Pressed`
    (`WorldGrid.Save` (`self.WorldGrid`))))

(fn `UserConstructionScript`)